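; AGR function library with shared helpers for forward line traces and for regenerating float values over time.
; AGRForwardTrace traces along a component's forward vector, using StartStop for the endpoints, by channel or object types, and returns whether it hit plus the hit result.
; AGRRegenFloat changes a by-ref float by a per-second rate scaled by world delta time and clamps it between min and max.
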(fn `AGR_ForwardTrace`
  (params (Component :type "SceneComponent Object Reference") (`ByChannel?` :type Boolean :default true) (TraceChannel :type "ETraceTypeQuery Enum" :default "TraceTypeQuery1") (ObjectTypes :type "Array of EObjectTypeQuery Enum (by ref)") (`TraceComplex?` :type Boolean) (TraceDistance :type "Float (double-precision)" :default 5000.0) (ActorsToIgnore :type "Array of Actor Object Reference (by ref)") (DrawDebugType :type "EDrawDebugTrace Enum" :default "None") (`IgnoreSelf?` :type Boolean :default true) (TraceColor :type "LinearColor Structure" :default (struct :`R` 1.0 :`A` 1.0)) (TraceHitColor :type "LinearColor Structure" :default (struct :`G` 1.0 :`A` 1.0)) (DrawTime :type "Float (double-precision)" :default 1.0))
  (returns (`GotHit?` :type Boolean) (OutHit :type "HitResult Structure"))
  (bind _returnvalue (`SceneComponent.K2_GetComponentLocation` Component))
  (bind _returnvalue_2 (+ _returnvalue (* (`SceneComponent.GetForwardVector` Component) TraceDistance)))
  (if `ByChannel?`
    (bind (_outhit _returnvalue_3) (`KismetSystemLibrary.LineTraceSingle` Component _returnvalue _returnvalue_2 TraceChannel `TraceComplex?` ActorsToIgnore DrawDebugType `IgnoreSelf?` TraceColor TraceHitColor DrawTime))
    (if _returnvalue_3
      (return true _outhit)
      (else
        (return false)))
    (else
      (bind (_outhit_2 _returnvalue_4) (`KismetSystemLibrary.LineTraceSingleForObjects` Component _returnvalue _returnvalue_2 ObjectTypes `TraceComplex?` ActorsToIgnore DrawDebugType `IgnoreSelf?` TraceColor TraceHitColor DrawTime))
      (if _returnvalue_4
        (return true _outhit_2)
        (else
          (return false))))))

(fn `AGR_RegenFloat`
  (params (Value :type "Float (double-precision) (by ref)") (PerSecond :type "Float (double-precision) (by ref)") (MIn :type "Float (double-precision) (by ref)") (Max :type "Float (double-precision) (by ref)"))
  (`|VariableSetRef` Value (`KismetMathLibrary.FClamp` (+ Value (* PerSecond (`GameplayStatics.GetWorldDeltaSeconds` null))) MIn Max)))