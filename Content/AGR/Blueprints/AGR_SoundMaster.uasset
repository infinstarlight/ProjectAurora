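; AGR_SoundMaster is a component that plays surface-dependent footstep sounds and Niagara particles for its owner, typically a Character.
; Named-foot calls, intended for notifies, or an optional Tick-based generator cycling through the feet trace down from foot sockets.
; The hit's physical surface, overridden by a water surface when InWater, keys the sound and particle maps.
; Velocity scales volume, sounds receive IsMale and Rattle parameters, and Setup events configure everything.
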(event `self.ReceiveBeginPlay`
  ;[0.7813 0 1] Begin Play
  (`KismetSystemLibrary.Delay` 0.0)
  (`self.EventGetOwnerAsCharacter`))

(event `EventGetOwnerAsCharacter`
  ;[0 1 0.2734] Check if owner is character for future reference
  (bind _ascharacter (cast `Character` (`self.GetOwner`))
    (:`then`
      (set `self.OwnerCharacterReference` _ascharacter))
    (:`CastFailed`
      (`KismetSystemLibrary.PrintString` "Error - owner is not a character!"))))

(event `EventSpawnSoundAttached`
  (params (Key :type "EPhysicalSurface Enum (by ref)") (Foot :type "Name (by ref)"))
  (bind _ownercharacterreference (`self.OwnerCharacterReference`))
  (bind (_value _returnvalue) (`BlueprintMapLibrary.Map_Find` (`self.SurfaceSounds`) Key))
  ;[1 0.5859 0] Spawn Sound
  (if _returnvalue
    (bind _returnvalue_2 (`GameplayStatics.SpawnSoundAttached` _value (select `bool` (`KismetSystemLibrary.IsValid` _ownercharacterreference) :`false` (`Actor.RootComponent` (`self.GetOwner`)) :`true` (`Character.Mesh` _ownercharacterreference) :!type "SceneComponent Object Reference") (`BlueprintMapLibrary.Map_Find` (`self.Feet`) Foot) (0.0 0.0 0.0) (struct) "SnapToTarget" false (* (`self.ReadVolumeValue` (`Actor.GetVelocity` (`self.GetOwner`))) (`self.VolumeMultiplier`)) 1.0 0.0 (`self.FootstepAttenuation`) (`self.FootstepConcurencySettings`)))
    ;;[0 0.9297 1] Parameters
    (`/Engine/EditorBlueprintResources/StandardMacros.IsValid` _returnvalue_2
      (:`Is Valid`
        (`AudioComponent.SetBoolParameter` _returnvalue_2 "IsMale" (`self.Male?`))
        (`AudioComponent.SetBoolParameter` _returnvalue_2 "Rattle" (`self.Rattle?`))))))

(event `SetupFootstepsDefaults`
  (params (VelocityToMinVolume :type "Float (double-precision)" :default 120.0) (VelocityMaxVolume :type "Float (double-precision)" :default 320.0) (`Male?` :type Boolean :default true) (`Rattle?` :type Boolean :default false) (VolumeMultiplier :type "Float (double-precision)" :default 1.0) (FootstepAttenuation :type "SoundAttenuation Object Reference") (FootstepConcurencySettings :type "SoundConcurrency Object Reference") (SurfaceSounds :type "Map of EPhysicalSurface Enum to SoundCue Object Reference") (SurfaceParticles :type "Map of EPhysicalSurface Enum to NiagaraSystem Object Reference") (`FootTraceComplex?` :type Boolean :default true) (FootstepsMinCycleInterval :type "Float (double-precision)" :default 0.25))
  ;[1 0 0.04687] Init setup
  (set `self.VelocityToMinVolume` VelocityToMinVolume)
  (set `self.VelocityMaxVolume` VelocityMaxVolume)
  (set `self.Male?` `Male?`)
  (set `self.Rattle?` `Rattle?`)
  (set `self.VolumeMultiplier` VolumeMultiplier)
  (set `self.FootstepAttenuation` FootstepAttenuation)
  (set `self.FootstepConcurencySettings` FootstepConcurencySettings)
  (set `self.SurfaceSounds` SurfaceSounds)
  (set `self.SurfaceParticles` SurfaceParticles)
  (set `self.FootTraceComplex?` `FootTraceComplex?`)
  (set `self.FootstepsMinCycleInterval` FootstepsMinCycleInterval))

(event `SetupFeetDefinition`
  (params (Feet :type "Map of Name to Name"))
  ;[0 1 0.7891] Setup definition of feet bone shortcuts for notification
  (set `self.Feet` Feet))

(event `EventTryFootstep`
  (params (FootsavedName :type Name) (Mesh :type "SkeletalMeshComponent Object Reference"))
  (bind (_found_ _socketname) (`self.FindSocketFromName` FootsavedName))
  (bind _debug_ (`self.Debug?`))
  ;[0 1 0.8828] Init Footstep Event
  (if (and _found_ (`SceneComponent.DoesSocketExist` Mesh _socketname))
    ;[0.5234 0 1] Trace foot
    (bind (_returnvalue _outhit _surface) (`self.TraceFoot` _socketname Mesh 30.0))
    ;[0.1016 0 1] Debug error print
    (if _returnvalue
      (`self.EventInitFootstep` _outhit _surface _socketname)
      (else
        (`KismetSystemLibrary.PrintString` "DebugPrint! Nothing under the feet" _debug_ _debug_ (struct :`G` 0.66 :`B` 1.0 :`A` 1.0) 0.5)))))

(event `SetupAddOrUpdateSurface`
  (params (Surface :type "EPhysicalSurface Enum" :default "SurfaceType_Default") (sound :type "SoundCue Object Reference (by ref)") (niagaraParticle :type "NiagaraSystem Object Reference (by ref)"))
  ;[0 0.625 1] Alter the surface setup
  (`BlueprintMapLibrary.Map_Add` (`self.SurfaceSounds`) Surface sound)
  (`BlueprintMapLibrary.Map_Add` (`self.SurfaceParticles`) Surface niagaraParticle))

(event `EventSpawnParticle`
  (params (Key :type "EPhysicalSurface Enum (by ref)") (Transform :type "Transform Structure"))
  (bind (_value _returnvalue) (`BlueprintMapLibrary.Map_Find` (`self.SurfaceParticles`) Key))
  ;[1 0 0.2344] Spawn Particle
  (if _returnvalue
    (`NiagaraFunctionLibrary.SpawnSystemAtLocation` _value Transform_Location Transform_Rotation Transform_Scale true true "AutoRelease")))

(event `self.ReceiveTick`
  (params (DeltaSeconds :type "Float (single-precision)"))
  (bind _ownercharacterreference (`self.OwnerCharacterReference`))
  (bind _autofootstepsarray (`self.AutofootstepsArray`))
  (bind _debug_ (`self.Debug?`))
  ;[0 0.7187 1] Tick auto footsteps generator!
  ;;[0 1 0.7891] Auto footstep generator
  (if (`self.AutoFootRotation?`)
    (bind _values (`BlueprintMapLibrary.Map_Values` (`self.Feet`)))
    (for _array_element _values
      ;;[0 1 0.25] PerFoot tracing
      (if (`KismetMathLibrary.BooleanNOR` (`KismetArrayLibrary.Array_Contains` _autofootstepsarray _array_element) (== (`self.PreviousFoot`) _array_element))
        (`/Engine/EditorBlueprintResources/StandardMacros.IsValid` _ownercharacterreference
          (:`Is Valid`
            (bind (_returnvalue _outhit _surface) (`self.TraceFoot` _array_element (`Character.Mesh` _ownercharacterreference) (`self.AutofootstepTraceLen`)))
            (if _returnvalue
              (`KismetArrayLibrary.Array_AddUnique` _autofootstepsarray _array_element)
              (`self.EventInitFootstep` _outhit _surface _array_element)
              (set `self.PreviousFoot` _array_element)))
          (:`Is Not Valid`
            (`self.EventGetOwnerAsCharacter`)))))
    ;;[1 0 0.3047] Clear on stop
    (if (== (`KismetArrayLibrary.Array_Length` (`self.AutofootstepsArray`)) (`KismetArrayLibrary.Array_Length` _values))
      (if (not (`KismetMathLibrary.NearlyEqual_FloatFloat` (`KismetMathLibrary.VSize` (`Actor.GetVelocity` (`self.OwnerCharacterReference`))) 0.0 0.01))
        (`/Engine/EditorBlueprintResources/StandardMacros.Gate` false :!label _label
          (:`Exit`
            (`KismetArrayLibrary.Array_Clear` (`self.AutofootstepsArray`))
            (`KismetSystemLibrary.PrintString` "cleared auto foot array!" _debug_ _debug_ (struct :`G` 0.66 :`B` 1.0 :`A` 1.0) 0.5)
            (`|ExecutionSequence`
              (:`then_0`
                (goto _label :!via `Close`))
              (:`then_1`
                (`KismetSystemLibrary.Delay` (`self.FootstepsMinCycleInterval`))
                (goto _label :!via `Open`)))))))))

(event `EventInitFootstep`
  (params (Hit :type "HitResult Structure (by ref)") (Key :type "EPhysicalSurface Enum (by ref)") (Foot :type "Name (by ref)"))
  (bind (_bblockinghit _binitialoverlap _time _distance _location _impactpoint _normal) (`GameplayStatics.BreakHitResult` Hit))
  ;[1 0.2109 0] The actual footstep Event
  ;;[0 1 0.1328] Init footstep
  (`|ExecutionSequence`
    (:`then_0`
      ;;[1 0.5625 0] Spawn Sound for footsteps
      (if (`self.UseFootstepSounds?`)
        (`self.EventSpawnSoundAttached` (select `bool` (`self.InWater?`) :`false` Key :`true` (`self.WaterSurface`)) Foot)))
    (:`then_1`
      ;;[0 1 1] Spawn Partickle
      (if (`self.UseFootstepParticle?`)
        (`self.EventSpawnParticle` (select `bool` (`self.InWater?`) :`false` Key :`true` (`self.WaterSurface`)) (`KismetMathLibrary.MakeTransform` _impactpoint (`KismetMathLibrary.Conv_VectorToRotator` _normal) (`Actor.GetActorScale3D` (`self.GetOwner`))))))
    (:`then_2`
      ;;[0 1 0.4844] Debug print
      (if (`self.Debug?`)
        (`KismetSystemLibrary.PrintText` (`|FormatText` "Footstep::     Surface:{0}   Foot:{1}" (`|GetEnumeratorNameAsString` Key) Foot) true true (struct :`G` 0.66 :`B` 1.0 :`A` 1.0) 0.5)))))

(event `SetupAutoFootsteps`
  (params (`AutoFootRotation?` :type Boolean :default true) (AutofootstepTraceLen :type "Float (double-precision)" :default 15.0))
  ;[0.6641 1 0] Setup auto footsteps
  (set `self.AutoFootRotation?` `AutoFootRotation?`)
  (set `self.AutofootstepTraceLen` AutofootstepTraceLen))

(event `SetupWaterSurface`
  (params (WaterSurface :type "EPhysicalSurface Enum" :default "SurfaceType3"))
  ;[1 0.1641 0] In Water
  (set `self.WaterSurface` WaterSurface))

(event `SetupInWater`
  (params (`InWater?` :type Boolean))
  ;[1 0.1641 0] In Water
  (set `self.InWater?` `InWater?`))

(fn `FindSocketFromName`
  (params (StoredFootName :type Name))
  (returns (`Found?` :type Boolean) (SocketName :type Name))
  (bind (_value _returnvalue) (`BlueprintMapLibrary.Map_Find` (`self.Feet`) StoredFootName))
  (return _returnvalue _value))

(fn `ReadVolumeValue`
  (params (InVelocity :type "Vector Structure"))
  (returns (OutVolume :type "Float (double-precision)"))
  (return (`KismetMathLibrary.MapRangeClamped` (`KismetMathLibrary.VSize` InVelocity) (`self.VelocityToMinVolume`) (`self.VelocityMaxVolume`) 0.1 1.0)))

(fn `TraceFoot`
  (params (TraceSocketName :type Name) (Mesh :type "SkeletalMeshComponent Object Reference") (TraceLen :type "Float (double-precision)"))
  (returns (ReturnValue :type Boolean) (OutHit :type "HitResult Structure") (Surface :type "EPhysicalSurface Enum") (ImpactPoint :type "Vector Structure"))
  (bind _returnvalue (`SceneComponent.GetSocketLocation` Mesh TraceSocketName))
  ;[1 0.7969 0] Trace
  (bind (_outhit _returnvalue_2) (`KismetSystemLibrary.LineTraceSingle` _returnvalue (+ _returnvalue (`KismetMathLibrary.MakeVector` 0.0 0.0 (* -1 TraceLen))) "TraceTypeQuery1" (`self.FootTraceComplex?`) (`|MakeArray` (`self.GetOwner`)) (select `bool` (`self.Debug?`) :`true` "ForDuration" :!type "EDrawDebugTrace Enum") true (struct :`R` 1.0 :`A` 1.0) (struct :`G` 1.0 :`A` 1.0) 1.0))
  ;[1 0 0] Got any hit
  (if _returnvalue_2
    ;[0.4062 1 0] Debug Draw
    (if (`self.Debug?`)
      (bind (_bblockinghit _binitialoverlap _time _distance _location _impactpoint _normal _impactnormal _physmat) (`GameplayStatics.BreakHitResult` _outhit))
      (`KismetSystemLibrary.DrawDebugSphere` _impactpoint 25.0 12 (struct :`G` 0.598958 :`B` 0.223925 :`A` 1.0) 0.5 1.0))
    (return _returnvalue_2 _outhit (`PhysicalMaterial.SurfaceType` _physmat) _impactpoint)
    (else
      (return false (struct) "SurfaceType_Default" (0.0 0.0 0.0)))))