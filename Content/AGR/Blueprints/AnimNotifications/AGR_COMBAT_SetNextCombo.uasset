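; Anim notify that queues the next attack in a melee combo while an attack animation plays.
; It finds the AGR_CombatMaster component on the mesh owner and passes it a key tag and follow-up montage via SetNextAttackInCombo.
; It prints a confirmation gated by that component's Debug flag, or a failure message if the component is missing.
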(fn `Received_Notify`
  (params (MeshComp :type "SkeletalMeshComponent Object Reference") (Animation :type "AnimSequenceBase Object Reference"))
  (returns (ReturnValue :type Boolean))
  (bind _key (`self.Key`))
  (bind _montage (`self.Montage`))
  (bind _returnvalue (`Actor.GetComponentByClass` (`ActorComponent.GetOwner` MeshComp) "/Game/AGR/Blueprints/AGR_CombatMaster.AGR_CombatMaster_C"))
  (bind _debug_ (`/Game/AGR/Blueprints/AGR_CombatMaster.Debug?` _returnvalue))
  (`/Engine/EditorBlueprintResources/StandardMacros.IsValid` _returnvalue
    (:`Is Valid`
      (`/Game/AGR/Blueprints/AGR_CombatMaster.SetNextAttackInCombo` _returnvalue _key _montage)
      (`KismetSystemLibrary.PrintText` (`|FormatText` "Combo Set! Button {0} - {1}" (`BlueprintGameplayTagLibrary.GetTagName` _key) _montage) _debug_ _debug_)
      (return true))
    (:`Is Not Valid`
      (`KismetSystemLibrary.PrintString` "Fail set combo")
      (return false))))