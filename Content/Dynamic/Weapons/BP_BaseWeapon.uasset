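; BP_BaseWeapon is a weapon base that exposes WeaponStats through getters and an attach-point setter, and fires hitscan shots.
; BeginPlay caches the owner, whose active camera supplies the trace origin and direction for FireWeapon.
; Standard and Incendiary share a single object trace that damages the hit actor; Hollow Point multi-traces, but its ApplyDamage has no target connected.
; CalculateDamage derives WeaponDamage from the stats, but nothing here calls it.
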(event `self.ReceiveBeginPlay`
  (bind _returnvalue (`self.GetOwner`))
  (`/Engine/EditorBlueprintResources/StandardMacros.IsValid` _returnvalue
    (:`Is Valid`
      (set `self.WeaponOwner` _returnvalue))))

(fn `CalculateDamage`
  (bind ((`BaseDamage_18_68FCAD9648DF6ACC1CA585BCB05D45ED` _basedamage) (`DamageMultiplier_21_B9BB9375418DCE94217468BFC40BF113` _damagemultiplier) (`DamageModifier_22_4DB9250742110AF603636AAF1E5064C6` _damagemodifier)) (break `/Game/Dynamic/Weapons/BP_FWeaponStats` (`self.WeaponStats`)))
  (set `self.WeaponDamage` (+ _basedamage (* _damagemultiplier _damagemodifier))))

(fn `FireWeapon`
  (bind _targetobjects (`self.TargetObjects`))
  (bind _camera (message `/Game/AGR/Blueprints/AGR_Interface.GetActiveCamera` (`self.WeaponOwner`)))
  (switch `/Game/Dynamic/Weapons/BP_EWeaponAmmoType` (`self.GetAmmoType`)
    (:`NewEnumerator0`
      (bind _returnvalue (`SceneComponent.K2_GetComponentLocation` _camera))
      (bind _returnvalue_2 (+ _returnvalue (* (`KismetMathLibrary.GetForwardVector` (`SceneComponent.K2_GetComponentRotation` _camera)) (`self.GetWeaponRange`))))
      (bind (_outhit _returnvalue_3) (`KismetSystemLibrary.LineTraceSingleForObjects` _returnvalue _returnvalue_2 _targetobjects true :!label _label))
      (if _returnvalue_3
        (bind (_bblockinghit _binitialoverlap _time _distance _location _impactpoint _normal _impactnormal _physmat _hitactor) (`GameplayStatics.BreakHitResult` _outhit))
        (`/Engine/EditorBlueprintResources/StandardMacros.IsValid` _hitactor
          (:`Is Valid`
            (`GameplayStatics.ApplyDamage` _hitactor (`self.WeaponDamage`))))))
    (:`NewEnumerator1`
      (bind (_outhits _returnvalue_4) (`KismetSystemLibrary.LineTraceMultiForObjects` _returnvalue _returnvalue_2 _targetobjects true))
      (if _returnvalue_4
        (for _array_element _outhits
          (`/Engine/EditorBlueprintResources/StandardMacros.IsValid` (`.HitActor` (`GameplayStatics.BreakHitResult` _array_element))
            (:`Is Valid`
              (`GameplayStatics.ApplyDamage` null (`self.WeaponDamage`)))))))
    (:`NewEnumerator2`
      (goto _label))))

(fn `GetAmmoType`
  (returns (ReturnValue :type "/Game/Dynamic/Weapons/BP_EWeaponAmmoType Enum"))
  (return (`.AmmoType_13_B2FC084A42F342726E1C40A0A50D15A7` (break `/Game/Dynamic/Weapons/BP_FWeaponStats` (`self.WeaponStats`)))))

(fn `GetAttachPoint`
  (returns (ReturnValue :type Name))
  (return (`.AttachPoint_28_8D33FCAD4FEFC61E1C4ED5A8CC5168B0` (break `/Game/Dynamic/Weapons/BP_FWeaponStats` (`self.WeaponStats`)))))

(fn `GetCurrentAmmo`
  (returns (CurrentMagAmmo :type Integer))
  (return (`.CurrentMagAmmo_4_ED441AAD42B32A7A854BDD8EA947EBAA` (break `/Game/Dynamic/Weapons/BP_FWeaponStats` (`self.WeaponStats`)))))

(fn `GetMagLimit`
  (returns (ReturnValue :type Integer))
  (return (`.MaxMagAmmo_5_64E747B04D3878E55B2DC38491204CA9` (break `/Game/Dynamic/Weapons/BP_FWeaponStats` (`self.WeaponStats`)))))

(fn `GetRoundType`
  (returns (ReturnValue :type "/Game/Dynamic/Weapons/BP_EWeaponRoundType Enum"))
  (return (`.RoundType_10_9E4985464DAA89CA4C9620B81947698D` (break `/Game/Dynamic/Weapons/BP_FWeaponStats` (`self.WeaponStats`)))))

(fn `GetWeaponRange`
  (returns (ReturnValue :type "Float (double-precision)"))
  (return (`.WeaponRange_16_AE16AE084F4C69CE9FA1EAB36F8DC3FC` (break `/Game/Dynamic/Weapons/BP_FWeaponStats` (`self.WeaponStats`)))))

(fn `GetWeaponType`
  (returns (ReturnValue :type "/Game/Dynamic/Weapons/BP_EWeaponType Enum"))
  (return (`.WeaponType_31_C10F874F436C92A437E7469E5D9E24DE` (break `/Game/Dynamic/Weapons/BP_FWeaponStats` (`self.WeaponStats`)))))

(fn `SetAttachPoint`
  (params (AttachPoint :type Name))
  (setmembers `/Game/Dynamic/Weapons/BP_FWeaponStats` :`StructRef` (`self.WeaponStats`) :`AttachPoint` AttachPoint))

(fn `UserConstructionScript`)